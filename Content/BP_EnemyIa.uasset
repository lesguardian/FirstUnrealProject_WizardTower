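; BP_EnemyIa is an enemy AI that wanders until it sees the player, then chases them.
; Patrol walks slowly to random reachable points within a radius, looping after a short pause on each successful move.
; When PawnSensing sees BP_Player it raises walk speed and moves toward that actor.
; A retriggerable delay refreshed by each sighting returns it to patrolling one second after the last one.
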(event `self.ReceiveBeginPlay`
  (`self.Patrol`))

(event `Patrol`
  (set `CharacterMovementComponent.MaxWalkSpeed` 200.0 (`self.CharacterMovement`))
  (`|AIMoveTo` self (`NavigationSystemV1.K2_GetRandomReachablePointInRadius` (`self.K2_GetActorLocation`) 1000.0 null null) null
    (:`OnSuccess`
      (`KismetSystemLibrary.Delay` 0.5)
      (`self.Patrol`))))

(event `self.PawnSensing.OnSeePawn`
  (params (Pawn :type "Pawn Object Reference"))
  (`|ExecutionSequence`
    (:`then_0`
      (bind _asbp_player (cast `/Game/BP_Player` Pawn))
      (set `CharacterMovementComponent.MaxWalkSpeed` 600.0 (`self.CharacterMovement`))
      (`|AIMoveTo` self (0.0 0.0 0.0) _asbp_player))
    (:`then_1`
      (`KismetSystemLibrary.RetriggerableDelay` 1.0)
      (`self.Patrol`))))

(fn `UserConstructionScript`)